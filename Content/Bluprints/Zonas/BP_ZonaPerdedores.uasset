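; BP_ZonaPerdedores is a zone actor that runs a three-phase "Tormenta" (storm) sequence, moving its phase components over time.
; BeginPlay chains delays set by the Fase variables, triggering each storm event in turn.
; Timelines drive Lerps on relative location: the first two components sink along Z and are destroyed when finished.
; The third component slides along X and remains in place.
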(event Custom|Tormenta%203
  (bind _down (Timeline|Timeline_1 Play)
    (:Update
      (Transformation|SetRelativeLocation (Variables|Default|GetP_Fase3) (Math|Vector|MakeVector (Math|Float|Lerp 0.0 1.5e+03 _down) 0.0 0.0) false false))))

(event Custom|Tormenta1
  (bind _p_fase1 (Variables|Default|GetP_Fase1))
  (bind _down (Timeline|Timeline Play)
    (:Update
      (Transformation|SetRelativeLocation _p_fase1 (Math|Vector|MakeVector 0.0 0.0 (Math|Float|Lerp 0.0 -1e+03 _down)) false false))
    (:Finished
      (Components|DestroyComponent _p_fase1))))

(event Custom|Tormenta%202
  (bind _p_fase2 (Variables|Default|GetP_Fase2))
  (bind _down (Timeline|Timeline_0 Play)
    (:Update
      (Transformation|SetRelativeLocation _p_fase2 (Math|Vector|MakeVector 0.0 0.0 (Math|Float|Lerp 0.0 -1e+03 _down)) false false))
    (:Finished
      (Components|DestroyComponent _p_fase2))))

(event EventBeginPlay
  (Utilities|FlowControl|Delay (Variables|Default|GetFase1))
  (CallFunction|Tormenta1)
  (Utilities|FlowControl|Delay (Variables|Default|GetFase2))
  (CallFunction|Tormenta2)
  (Utilities|FlowControl|Delay (Variables|Default|GetFase3))
  (CallFunction|Tormenta3))

(event Collision|EventActorBeginOverlap
  (params (OtherActor :type Actor%20Object%20Reference)))

(event EventTick
  (params (DeltaSeconds :type Float%20%28single-precision%29)))

(fn ConstructionScript)