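; BP_Placa is a pressure plate that activates while the third-person character or a BP_CubeTest2 actor overlaps its sphere trigger.
; After a short delay, overlap begin plays a sound, sets IsActive and runs the Down timeline to lower the plate mesh.
; Overlap end clears IsActive after the same delay and reverses the timeline, without counting any other actors still on the plate.
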(event OnComponentBeginOverlap(Sphere)
  (params (OverlappedComponent :type Primitive%20Component%20Object%20Reference) (OtherActor :type Actor%20Object%20Reference) (OtherComp :type Primitive%20Component%20Object%20Reference) (OtherBodyIndex :type Integer) (bFromSweep :type Boolean) (SweepResult :type Hit%20Result%20Structure%20%28by%20ref%29))
  (Utilities|FlowControl|Sequence
    (:then_0
      (Utilities|Casting|CastToBP_ThirdPersonCharacter OtherActor))
    (:then_1
      (Utilities|Casting|CastToBP_CubeTest2 OtherActor)))
  (Utilities|FlowControl|Delay 0.2)
  (Audio|PlaySoundatLocation 0 (Transformation|GetActorLocation) "0, 0, 0" 1.0 1.0 0.0 0 0 0 0)
  (Variables|Default|SetIs%20Active? true)
  (bind _down (Timeline|Down Play)
    (:Update
      (Transformation|SetRelativeLocation (Variables|Default|GetPleasurePlate) (Math|Vector|MakeVector 0.0 0.0 (Math|Float|Lerp 1e+01 3.0 _down)) false false))))

(event OnComponentEndOverlap(Sphere)
  (params (OverlappedComponent :type Primitive%20Component%20Object%20Reference) (OtherActor :type Actor%20Object%20Reference) (OtherComp :type Primitive%20Component%20Object%20Reference) (OtherBodyIndex :type Integer))
  (Utilities|FlowControl|Sequence
    (:then_0
      (Utilities|Casting|CastToBP_ThirdPersonCharacter OtherActor))
    (:then_1
      (Utilities|Casting|CastToBP_CubeTest2 OtherActor)))
  (Utilities|FlowControl|Delay 0.2)
  (Variables|Default|SetIs%20Active? false)
  (bind _down (Timeline|Down Reverse)
    (:Update
      (Transformation|SetRelativeLocation (Variables|Default|GetPleasurePlate) (Math|Vector|MakeVector 0.0 0.0 (Math|Float|Lerp 1e+01 3.0 _down)) false false))))

(event EventBeginPlay)

(event Collision|EventActorBeginOverlap
  (params (OtherActor :type Actor%20Object%20Reference)))

(event EventTick
  (params (DeltaSeconds :type Float%20%28single-precision%29)))

(fn ConstructionScript)